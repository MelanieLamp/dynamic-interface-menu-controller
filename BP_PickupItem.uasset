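; BP_PickupItem is a world pickup that adds its ItemDefinition to the inventory of whatever actor overlaps it.
; The construction script reads the definition's WorldRepresentation fragment to set the static mesh, so the pickup's look follows its item data.
; On overlap it looks for an InventoryManagerComponent on the other actor, calls AddItem with the definition, then destroys itself.
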(event EventBeginPlay)

(event Collision|EventActorBeginOverlap
  (params (OtherActor :type Actor%20Object%20Reference))
  (bind _returnvalue (Actor|GetComponentbyClass OtherActor "/Game/01_MyContent/InventorySystem/InventoryManagerComponent.InventoryManagerComponent_C"))
  (Utilities|IsValid _returnvalue
    (:Is%20Valid
      (Default|AddItem _returnvalue (Variables|Default|GetItemDefinition))
      (Actor|DestroyActor))))

(fn ConstructionScript
  (bind _itemdefinition (Variables|Default|GetItemDefinition))
  (bind _returnvalue (Class|ItemDefinition|FindFragmentbyClass _itemdefinition "/Script/MyPractice.InventoryItemFragment_WorldRepresentation"))
  (Utilities|IsValid _returnvalue
    (:Is%20Valid
      (Components|StaticMesh|SetStaticMesh (Variables|Default|GetStaticMesh) (Variables|/Script/MyPractice.InventoryItemFragment_WorldRepresentation|GetItemMesh _returnvalue)))))